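; BP_Enemy is a patrolling enemy that chases the player once spotted and restarts the current level when it touches them.
; From BeginPlay, a timeline moves it along a Path spline, setting location and rotation by interpolated distance.
; Player overlap with a cone shape sets a never-cleared seen flag, after which Tick stops the timeline and issues AIMoveTo toward the player every frame.
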(event OnComponentBeginOverlap(Shape_Cone1)
  (params (OverlappedComponent :type Primitive%20Component%20Object%20Reference) (OtherActor :type Actor%20Object%20Reference) (OtherComp :type Primitive%20Component%20Object%20Reference) (OtherBodyIndex :type Integer) (bFromSweep :type Boolean) (SweepResult :type Hit%20Result%20Structure%20%28by%20ref%29))
  (Utilities|Casting|CastToBP_Character OtherActor)
  (Variables|Default|SetIsSeeingPlayer true))

(event OnComponentBeginOverlap(CapsuleComponent)
  (params (OverlappedComponent :type Primitive%20Component%20Object%20Reference) (OtherActor :type Actor%20Object%20Reference) (OtherComp :type Primitive%20Component%20Object%20Reference) (OtherBodyIndex :type Integer) (bFromSweep :type Boolean) (SweepResult :type Hit%20Result%20Structure%20%28by%20ref%29))
  (Utilities|Casting|CastToBP_Character OtherActor
    (:then
      (bind _returnvalue (Game|GetCurrentLevelName true))
      (Game|OpenLevel(byName) (Utilities|String|StringToName _returnvalue)))
    (:CastFailed
      (Development|PrintString "Colliding with non-player"))))

(event Custom|FollowPlayer
  (AI|AIMoveTo self "0, 0, 0" (Game|GetPlayerCharacter 0) 5.0 false))

(event Custom|FollowPath
  (bind _alpha (Timeline|Timeline Play)
    (:Update
      (Transformation|SetActorLocationAndRotation (.location (Spline|GetTransformatDistanceAlongSpline (Variables|/Game/Enemy/BP_Path.BP_Path_C|GetSpline (Variables|Default|GetPath)) (Math|Float|Lerp 0.0 (Spline|GetSplineLength (Variables|/Game/Enemy/BP_Path.BP_Path_C|GetSpline (Variables|Default|GetPath))) _alpha) "World" false)) (.rotation (Spline|GetTransformatDistanceAlongSpline (Variables|/Game/Enemy/BP_Path.BP_Path_C|GetSpline (Variables|Default|GetPath)) (Math|Float|Lerp 0.0 (Spline|GetSplineLength (Variables|/Game/Enemy/BP_Path.BP_Path_C|GetSpline (Variables|Default|GetPath))) _alpha) "World" false))))))

(event EventBeginPlay
  (CallFunction|FollowPath))

(event Collision|EventActorBeginOverlap
  (params (OtherActor :type Actor%20Object%20Reference)))

(event EventTick
  (params (DeltaSeconds :type Float%20%28single-precision%29))
  (if (Variables|Default|GetIsSeeingPlayer)
    (CallFunction|FollowPlayer)
    (bind _alpha (Timeline|Timeline Stop)
      (:Update
        (Transformation|SetActorLocationAndRotation (.location (Spline|GetTransformatDistanceAlongSpline (Variables|/Game/Enemy/BP_Path.BP_Path_C|GetSpline (Variables|Default|GetPath)) (Math|Float|Lerp 0.0 (Spline|GetSplineLength (Variables|/Game/Enemy/BP_Path.BP_Path_C|GetSpline (Variables|Default|GetPath))) _alpha) "World" false)) (.rotation (Spline|GetTransformatDistanceAlongSpline (Variables|/Game/Enemy/BP_Path.BP_Path_C|GetSpline (Variables|Default|GetPath)) (Math|Float|Lerp 0.0 (Spline|GetSplineLength (Variables|/Game/Enemy/BP_Path.BP_Path_C|GetSpline (Variables|Default|GetPath))) _alpha) "World" false)))))))

(fn ConstructionScript)