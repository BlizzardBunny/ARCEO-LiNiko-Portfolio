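; Player character Blueprint that handles Enhanced Input movement, camera look with optional axis inversion, jumping, interaction and quitting.
; On BeginPlay it adds the input mapping context and shows a WASD hint widget, which the move input removes.
; Each Tick, a short line trace from the camera finds an interactable BP_Interactable, stores it and shows its UI.
; The interact input triggers the stored target, which is cleared when the trace no longer hits an interactable.
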(event Input|EnhancedActionEvents|EnhancedInputActionINP_Jump
  (params (ActionValue :type Boolean) (ElapsedSeconds :type Float%20%28double-precision%29) (TriggeredSeconds :type Float%20%28double-precision%29) (InputAction :type Input%20Action%20Object%20Reference :default "/Game/PlayerCharacter/INP_Jump.INP_Jump"))
  (:Started
    (Character|Jump))
  (:Completed
    (Character|StopJumping)))

(event Input|EnhancedActionEvents|EnhancedInputActionINP_MoveAround
  (params (ActionValue :type Vector%202D%20Structure) (ElapsedSeconds :type Float%20%28double-precision%29) (TriggeredSeconds :type Float%20%28double-precision%29) (InputAction :type Input%20Action%20Object%20Reference :default "/Game/PlayerCharacter/INP_MoveAround.INP_MoveAround"))
  (bind _returnvalue (Pawn|GetControlRotation :!class /Script/Engine.Pawn))
  (Pawn|Input|AddMovementInput (Math|Vector|GetRightVector (Pawn|GetControlRotation :!class /Script/Engine.Pawn)) (.x ActionValue) false)
  (Pawn|Input|AddMovementInput (Math|Vector|GetForwardVector (Math|Rotator|MakeRotator (.roll _returnvalue) 0.0 (.yaw _returnvalue))) (.y ActionValue) false)
  (Widget|RemovefromParent (Variables|Default|GetWASDWidget)))

(event Input|EnhancedActionEvents|EnhancedInputActionINP_LookAround
  (params (ActionValue :type Vector%202D%20Structure) (ElapsedSeconds :type Float%20%28double-precision%29) (TriggeredSeconds :type Float%20%28double-precision%29) (InputAction :type Input%20Action%20Object%20Reference :default "/Game/PlayerCharacter/INP_LookAround.INP_LookAround"))
  (Pawn|Input|AddControllerYawInput (* (.x ActionValue) (Math|Float|SelectFloat -1.0 1.0 (Variables|Default|GetInvertCameraX))))
  (Pawn|Input|AddControllerPitchInput (* (.y ActionValue) (Math|Float|SelectFloat -1.0 1.0 (Variables|Default|GetInvertCameraY)))))

(event Input|EnhancedActionEvents|EnhancedInputActionINP_Interact
  (params (ActionValue :type Boolean) (ElapsedSeconds :type Float%20%28double-precision%29) (TriggeredSeconds :type Float%20%28double-precision%29) (InputAction :type Input%20Action%20Object%20Reference :default "/Game/PlayerCharacter/INP_Interact.INP_Interact"))
  (bind _currentinteractable (Variables|Default|GetCurrentInteractable))
  (:Started
    (Utilities|IsValid _currentinteractable
      (:Is%20Valid
        (Default|BeginInteraction _currentinteractable)))))

(event Input|EnhancedActionEvents|EnhancedInputActionINP_Exit
  (params (ActionValue :type Boolean) (ElapsedSeconds :type Float%20%28double-precision%29) (TriggeredSeconds :type Float%20%28double-precision%29) (InputAction :type Input%20Action%20Object%20Reference :default "/Game/PlayerCharacter/INP_Exit.INP_Exit"))
  (:Started
    (Game|QuitGame 0 "Quit" false)))

(event EventBeginPlay
  (bind _returnvalue (Game|GetPlayerController 0))
  (bind _returnvalue_2 (PlayerController|LocalPlayerSubsystems|GetEnhancedInputLocalPlayerSubsystem _returnvalue))
  (Utilities|IsValid _returnvalue_2
    (:Is%20Valid
      (Input|AddMappingContext _returnvalue_2 "/Game/PlayerCharacter/INC_ThirdPerson.INC_ThirdPerson" 0 "(bIgnoreAllPressedKeysUntilRelease=True,bForceImmediately=False,bNotifyUserSettings=False)")
      (bind _returnvalue_3 (UserInterface|CreateWidget "/Game/PlayerCharacter/UI_WASD.UI_WASD_C"))
      (bind _output_get (Variables|Default|SetWASDWidget _returnvalue_3))
      (UserInterface|Viewport|AddtoViewport _output_get 0))))

(event Collision|EventActorBeginOverlap
  (params (OtherActor :type Actor%20Object%20Reference)))

(event EventTick
  (params (DeltaSeconds :type Float%20%28single-precision%29))
  (bind _playercamera (Variables|Default|GetPlayerCamera))
  (bind _returnvalue (Transformation|GetWorldLocation _playercamera))
  (bind _outhit (Collision|LineTraceByChannel _returnvalue (+ _returnvalue (* (Math|Vector|GetForwardVector (Transformation|GetWorldRotation _playercamera)) 2.5e+02)) "TraceTypeQuery1" false 0 "None"))
  (bind _asbp_interactable (Utilities|Casting|CastToBP_Interactable (.HitActor (Collision|BreakHitResult _outhit)))
    (:then
      (if (Variables|/Game/Interactables/BP_Interactable.BP_Interactable_C|GetCanInteract _asbp_interactable)
        (bind _output_get (Variables|Default|SetCurrentInteractable _asbp_interactable))
        (UserInterface|Viewport|AddtoViewport (Variables|/Game/Interactables/BP_Interactable.BP_Interactable_C|GetUI _output_get) 0)))
    (:CastFailed
      (Utilities|IsValid (Variables|Default|GetCurrentInteractable)
        (:Is%20Valid
          (Widget|RemovefromParent (Variables|/Game/Interactables/BP_Interactable.BP_Interactable_C|GetUI (Variables|Default|GetCurrentInteractable)))
          (Variables|Default|SetCurrentInteractable 0))))))

(fn ConstructionScript)